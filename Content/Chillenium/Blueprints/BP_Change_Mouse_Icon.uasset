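; BP_Change_Mouse_Icon is an actor that shows a flipbook icon at the mouse cursor for the currently selected item, such as bomb, vial, bubblegum, acid barrel or cinderblock.
; Each Tick switches on MouseValue to set the Flipbook, clearing it for the default value.
; For item values, it also moves the actor to the deprojected mouse world location of player 0.
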(event EventBeginPlay)

(event Collision|EventActorBeginOverlap
  (params (OtherActor :type Actor%20Object%20Reference)))

(event EventTick
  (params (DeltaSeconds :type Float%20%28single-precision%29))
  (switch int (Variables|Default|GetMouse%20Value)
    (:0
      ;[1 1 1] Default Cursor
      (Sprite|SetFlipbook (Variables|Default|GetFlipbook)))
    (:1
      ;[1 1 1] Comment
      (Sprite|SetFlipbook (Variables|Default|GetFlipbook) "/Game/Chillenium/Sprites/FB_Click_Bomb.FB_Click_Bomb")
      (Transformation|SetActorLocation (.WorldLocation (Game|Player|ConvertMouseLocationToWorldSpace (Game|GetPlayerController 0))) false false))
    (:2
      ;[1 1 1] Wall
      (Sprite|SetFlipbook (Variables|Default|GetFlipbook) "/Game/Chillenium/Flipbook/FB_Vial.FB_Vial")
      (Transformation|SetActorLocation (.WorldLocation (Game|Player|ConvertMouseLocationToWorldSpace (Game|GetPlayerController 0))) false false))
    (:3
      ;[1 1 1] Bounce
      (Sprite|SetFlipbook (Variables|Default|GetFlipbook) "/Game/Chillenium/Flipbook/FB_Bubblegum.FB_Bubblegum")
      (Transformation|SetActorLocation (.WorldLocation (Game|Player|ConvertMouseLocationToWorldSpace (Game|GetPlayerController 0))) false false))
    (:4
      ;[1 1 1] Acid Barrel
      (Sprite|SetFlipbook (Variables|Default|GetFlipbook) "/Game/Chillenium/Flipbook/FB_AcidBarrel.FB_AcidBarrel")
      (Transformation|SetActorLocation (.WorldLocation (Game|Player|ConvertMouseLocationToWorldSpace (Game|GetPlayerController 0))) false false))
    (:5
      ;[1 1 1] Bridge
      (Sprite|SetFlipbook (Variables|Default|GetFlipbook) "/Game/Chillenium/Flipbook/FB_Cinderblock.FB_Cinderblock")
      (Transformation|SetActorLocation (.WorldLocation (Game|Player|ConvertMouseLocationToWorldSpace (Game|GetPlayerController 0))) false false))))

(fn ConstructionScript)