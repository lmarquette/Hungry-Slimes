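; Lemmings-style slime character that walks sideways, flipping direction when stalled, until an ability event transforms it.
; Tick drives movement, facing and a non-looping random MultiGate that leaves each slime a random colour.
; Ability events stop it, show an emote and smoke, then replace it with a bridge, wall, bounce pad or acid slime, or explode nearby BombableBlock actors.
; Each loss decrements BP_Spawn_Slime's SlimeLives and updates BP_Mouse.
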(event Custom|Killing%20Slimes
  ;[1 1 1] Lower Slime Counter
  (bind _outactors (Actor|GetAllActorsOfClass "/Game/Chillenium/Blueprints/BP_Spawn_Slime.BP_Spawn_Slime_C"))
  (bind _asbp_spawn_slime (Utilities|Casting|CastToBP_Spawn_Slime (Utilities|Array|Get(acopy) _outactors)))
  (bind _output_get (Variables|/Game/Chillenium/Blueprints/BP_Spawn_Slime.BP_Spawn_Slime_C|SetSlime%20Lives _asbp_spawn_slime (- (Variables|/Game/Chillenium/Blueprints/BP_Spawn_Slime.BP_Spawn_Slime_C|GetSlime%20Lives _asbp_spawn_slime) 1.0)))
  (bind _asbp_mouse (Utilities|Casting|CastToBP_Mouse (Game|GetPlayerController 0)))
  (Default|SetSlimeLives _asbp_mouse _output_get))

(event Custom|UpdateAnimation
  ;[1 1 1] Handle Animation
  (Utilities|FlowControl|MultiGate true false -1
    (:Out%200
      ;;[1 1 1] Pink Slime
      (Sprite|SetFlipbook (Variables|Default|GetSprite) (select (> (Math|Vector|VectorLength (Transformation|GetVelocity)) 0.0) "/Game/Chillenium/Flipbook/FB_PinkSlime.FB_PinkSlime" "/Game/Chillenium/Flipbook/FB_PinkSlime.FB_PinkSlime"))
      (Audio|PlaySound2D "/Game/Chillenium/Sound/188384__wubitog__slime-attack-or-movement.188384__wubitog__slime-attack-or-movement" 1.0 1.0 0.0 0 0))
    (:Out%201
      ;;[1 1 1] Blue Slime
      (Sprite|SetFlipbook (Variables|Default|GetSprite) (select (> (Math|Vector|VectorLength (Transformation|GetVelocity)) 0.0) "/Game/Chillenium/Flipbook/FB_RedSlime.FB_RedSlime" "/Game/Chillenium/Flipbook/FB_RedSlime.FB_RedSlime")))
    (:Out%202
      ;;[1 1 1] Red Slime
      (Sprite|SetFlipbook (Variables|Default|GetSprite) (select (> (Math|Vector|VectorLength (Transformation|GetVelocity)) 0.0) "/Game/Chillenium/Flipbook/FB_Blueslime.FB_Blueslime" "/Game/Chillenium/Flipbook/FB_Blueslime.FB_Blueslime")))
    (:Out%203
      ;;[1 1 1] Yellow Slime
      (Sprite|SetFlipbook (Variables|Default|GetSprite) (select (> (Math|Vector|VectorLength (Transformation|GetVelocity)) 0.0) "/Game/Chillenium/Flipbook/FB_YellowSlime.FB_YellowSlime" "/Game/Chillenium/Flipbook/FB_YellowSlime.FB_YellowSlime")))
    (:Out%204
      ;;[1 1 1] Green Slime
      (Sprite|SetFlipbook (Variables|Default|GetSprite) (select (> (Math|Vector|VectorLength (Transformation|GetVelocity)) 0.0) "/Game/Chillenium/Flipbook/FB_GreenSlime.FB_GreenSlime" "/Game/Chillenium/Flipbook/FB_GreenSlime.FB_GreenSlime")))))

(event Custom|TrampolineSlime
  (bind _capsulecomponent (Variables|Collision|GetCapsuleComponent))
  (bind _returnvalue (Transformation|GetWorldTransform _capsulecomponent))
  ;[1 1 1] Trampoline Slime
  (Variables|Default|SetMovement 0.0)
  (bind _returnvalue_2 (Game|SpawnActorfromClass "/Game/Chillenium/Blueprints/BP_Question.BP_Question_C" (Math|Transform|MakeTransform (Math|Vector|MakeVector (+ (.x (.location _returnvalue)) 5.0) 0.0 (+ (.z (.location _returnvalue)) 5.0)) "0, 0, 0" "1,1,1") "Undefined" 0 0))
  (Utilities|FlowControl|Delay 0.4)
  (Actor|DestroyActor _returnvalue_2)
  (Sprite|SetFlipbook (Variables|Default|GetSprite) "/Game/Chillenium/Flipbook/FB_Smoke.FB_Smoke")
  (Variables|Default|SetIsSpecialAnimating true)
  (Utilities|FlowControl|Delay 0.5)
  (Game|SpawnActorfromClass "/Game/Chillenium/Items_For_Slime_To_Absorb/SlimeBouncePad.SlimeBouncePad_C" (Transformation|GetActorTransform) "Undefined" 0 0)
  (Actor|DestroyActor)
  (CallFunction|KillingSlimes))

(event Custom|AcidMelt
  (bind _capsulecomponent (Variables|Collision|GetCapsuleComponent))
  (bind _returnvalue (Transformation|GetWorldTransform _capsulecomponent))
  ;[1 1 1] Acid Melt
  (Variables|Default|SetMovement 0.0)
  (bind _returnvalue_2 (Game|SpawnActorfromClass "/Game/Chillenium/Blueprints/BP_Crying.BP_Crying_C" (Math|Transform|MakeTransform (Math|Vector|MakeVector (+ (.x (.location _returnvalue)) 5.0) 0.0 (.z (.location _returnvalue))) "0, 0, 0" "1,1,1") "Undefined" 0 0))
  (Utilities|FlowControl|Delay 0.5)
  (Actor|DestroyActor _returnvalue_2)
  (Sprite|SetFlipbook (Variables|Default|GetSprite) "/Game/Chillenium/Flipbook/FB_Smoke.FB_Smoke")
  (Audio|PlaySound2D "/Game/Chillenium/Sound/202094__spookymodem__acid-bubbling.202094__spookymodem__acid-bubbling" 1.0 1.0 0.0 0 0)
  (Variables|Default|SetIsSpecialAnimating true)
  (Utilities|FlowControl|Delay 0.3)
  (Game|SpawnActorfromClass "/Game/Chillenium/Blueprints/BP_Acid_Slime.BP_Acid_Slime_C" (Transformation|GetActorTransform) "Undefined" 0 0)
  (Actor|DestroyActor)
  (CallFunction|KillingSlimes))

(event Custom|Spawn%20Slime
  ;[1 1 1] Spawn Slimes
  (Game|SpawnActorfromClass "BP_Slime_C" (Transformation|GetWorldTransform (Variables|Collision|GetCapsuleComponent)) "AlwaysSpawn" 0 0))

(event Custom|Transform%20Slime%20into%20Wall
  (bind _capsulecomponent (Variables|Collision|GetCapsuleComponent))
  (bind _returnvalue (Transformation|GetWorldTransform _capsulecomponent))
  ;[1 1 1] SlimeWall
  (Utilities|FlowControl|DoOnce false
    (:Completed
      (Variables|Default|SetMovement 0.0)
      (bind _returnvalue_2 (Game|SpawnActorfromClass "/Game/Chillenium/Blueprints/BP_Question.BP_Question_C" (Math|Transform|MakeTransform (Math|Vector|MakeVector (+ (.x (.location _returnvalue)) 5.0) 0.0 (+ (.z (.location _returnvalue)) 5.0)) "0, 0, 0" "1,1,1") "Undefined" 0 0))
      (Utilities|FlowControl|Delay 0.5)
      (Sprite|SetFlipbook (Variables|Default|GetSprite) "/Game/Chillenium/Flipbook/FB_Smoke.FB_Smoke")
      (Audio|PlaySound2D "/Game/Chillenium/Sound/185831__lloydevans09__squeezy-squeaker.185831__lloydevans09__squeezy-squeaker" 1.0 1.0 0.0 0 0)
      (Actor|DestroyActor _returnvalue_2)
      (Variables|Default|SetIsSpecialAnimating true)
      (Utilities|FlowControl|Delay 0.4)
      (Utilities|FlowControl|Sequence
        (:then_0
          (Game|SpawnActorfromClass "/Game/Chillenium/Items_For_Slime_To_Absorb/SlimeWall.SlimeWall_C" (Transformation|GetWorldTransform (Variables|Collision|GetCapsuleComponent)) "AlwaysSpawn" 0 0))
        (:then_1
          (Actor|DestroyActor)
          (CallFunction|KillingSlimes))))))

(event Custom|GotBomb
  (bind _capsulecomponent (Variables|Collision|GetCapsuleComponent))
  (bind _returnvalue (Transformation|GetWorldTransform _capsulecomponent))
  ;[1 1 1] Bomb
  (Utilities|FlowControl|DoOnce false
    (:Completed
      (Variables|Default|SetMovement 0.0)
      (bind _returnvalue_2 (Game|SpawnActorfromClass "/Game/Chillenium/Blueprints/BP_Eclamation.BP_Eclamation_C" (Math|Transform|MakeTransform (Math|Vector|MakeVector (+ (.x (.location _returnvalue)) 5.0) 0.0 (+ (.z (.location _returnvalue)) 5.0)) "0, 0, 0" "1,1,1") "Undefined" 0 0))
      (Utilities|FlowControl|Delay 0.5)
      (Actor|DestroyActor _returnvalue_2)
      (Sprite|SetFlipbook (Variables|Default|GetSprite) "/Game/Chillenium/Flipbook/FB_Smoke.FB_Smoke")
      (Audio|PlaySound2D "/Game/Chillenium/Sound/369529__johandeecke__medium-explosion.369529__johandeecke__medium-explosion" 1.0 1.0 0.0 0 0)
      (Utilities|FlowControl|Delay 0.5)
      (bind _output_get (Variables|Default|SetIsSpecialAnimating true))
      (Variables|Default|SetIsBombing _output_get))))

(event Custom|SlimeBridge
  (bind _capsulecomponent (Variables|Collision|GetCapsuleComponent))
  (bind _returnvalue (Transformation|GetWorldTransform _capsulecomponent))
  ;[1 1 1] SlimeBridge
  (Utilities|FlowControl|DoOnce false
    (:Completed
      (Variables|Default|SetMovement 0.0)
      (bind _returnvalue_2 (Game|SpawnActorfromClass "/Game/Chillenium/Blueprints/BP_Question.BP_Question_C" (Math|Transform|MakeTransform (Math|Vector|MakeVector (+ (.x (.location _returnvalue)) 5.0) 0.0 (+ (.z (.location _returnvalue)) 5.0)) "0, 0, 0" "1,1,1") "Undefined" 0 0))
      (Utilities|FlowControl|Delay 0.5)
      (Sprite|SetFlipbook (Variables|Default|GetSprite) "/Game/Chillenium/Flipbook/FB_Smoke.FB_Smoke")
      (Audio|PlaySound2D "/Game/Chillenium/Sound/185831__lloydevans09__squeezy-squeaker.185831__lloydevans09__squeezy-squeaker" 1.0 1.0 0.0 0 0)
      (Actor|DestroyActor _returnvalue_2)
      (Variables|Default|SetIsSpecialAnimating true)
      (Utilities|FlowControl|Delay 0.4)
      (Utilities|FlowControl|Sequence
        (:then_0
          (Game|SpawnActorfromClass "/Game/Chillenium/Items_For_Slime_To_Absorb/BridgeSlime.BridgeSlime_C" (Transformation|GetWorldTransform (Variables|Collision|GetCapsuleComponent)) "AlwaysSpawn" 0 0))
        (:then_1
          (Actor|DestroyActor)
          (CallFunction|KillingSlimes))))))

(event EventTick
  (params (DeltaSeconds :type Float%20%28single-precision%29))
  ;[1 1 1] Tick - Updates animation
  (if (Variables|Default|GetIsSpecialAnimating)
    (if (Variables|Default|GetIsBombing)
      (for _array_element (Collision|GetOverlappingActors (Variables|Default|GetSphere) 0 :!class /Script/Engine.PrimitiveComponent)
        (if (Actor|ActorHasTag _array_element "BombableBlock")
          (Actor|DestroyActor _array_element)))
      (Utilities|FlowControl|Delay 0.1)
      (Actor|DestroyActor)
      (CallFunction|KillingSlimes))
    (else
      (Utilities|FlowControl|Sequence
        (:then_0
          (Pawn|Input|AddMovementInput "1.000000,0.000000, 0" (Variables|Default|GetMovement) false)
          (if (< (Math|Vector|VectorLength (Transformation|GetVelocity)) 1.0)
            (Utilities|FlowControl|FlipFlop
              (:A
                (Variables|Default|SetMovement (* (Variables|Default|GetMovement) -1.0)))
              (:B
                (Variables|Default|SetMovement (* (Variables|Default|GetMovement) 1.0))))))
        (:then_1
          (CallFunction|UpdateAnimation)
          (Math|Float|CompareFloat (.X (Math|Vector|BreakVector (Variables|/Script/Engine.MovementComponent|GetVelocity (Pawn|GetMovementComponent)))) 0.0
            (:>
              (Transformation|SetActorRotation (Math|Rotator|MakeRotator 0.0 0.0 0.0) :!label _label))
            (:==
              (if (Variables|Default|GetbisMovingRight)
                (goto _label)
                (else
                  (Transformation|SetActorRotation (Math|Rotator|MakeRotator 0.0 0.0 1.8e+02) :!label _label_2))))
            (:<
              (goto _label_2))))))))

(event EventBeginPlay
  (Class|ActorComponent|SetIsReplicated (Variables|Default|GetSprite) true))

(event Input|AxisEvents|InputAxisMoveRight
  (params (AxisValue :type Float%20%28single-precision%29))
  ;[1 1 1] Handle movement
)

(fn ConstructionScript)