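; BP_Spawn_Slime is a spawner that creates a limited number of BP_Slime AI pawns at its root location.
; Tick feeds an initially open Gate that closes after each spawn, then reopens after a short Delay and a SlimeCounter increment.
; When the counter equals SlimeLives, set on BeginPlay, it sets AllSlimeSpawned and leaves the Gate closed.
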(event Collision|EventActorBeginOverlap
  (params (OtherActor :type Actor%20Object%20Reference)))

(event EventTick
  (params (DeltaSeconds :type Float%20%28single-precision%29))
  (Utilities|FlowControl|Gate false :!label _label
    (:Exit
      (AI|SpawnAIFromClass "/Game/Chillenium/Blueprints/BP_Slime.BP_Slime_C" 0 (Transformation|GetWorldLocation (Variables|Default|GetDefaultSceneRoot)) "0, 0, 0" false)
      (Utilities|FlowControl|Sequence
        (:then_0
          (goto _label Close))
        (:then_1
          (if (== (Variables|Default|GetSlime%20Counter) (Variables|Default|GetSlime%20Lives))
            (Variables|Default|SetAll%20Slime%20Spawned true)
            (goto _label Close)
            (else
              (Utilities|FlowControl|Delay 2.0)
              (Variables|Default|SetSlime%20Counter (+ (Variables|Default|GetSlime%20Counter) 1.0))
              (goto _label Open))))))))

(event EventBeginPlay
  (Variables|Default|SetSlime%20Lives 5.0))

(fn ConstructionScript)