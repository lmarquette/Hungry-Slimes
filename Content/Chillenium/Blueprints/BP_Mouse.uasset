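; BP_Mouse places the selected slime or object (bomb, wall, bounce, acid, bridge) at the cursor on left-click release.
; It reads MouseValue from the BP_Change_Mouse_Icon actor to pick the class, then resets it to 0 after spawning.
; Spawns use the cursor trace's X and Z with Y left at zero, suggesting side-view play.
; It also creates the slimes-available UI when enabled, forwards life updates to it, and can restart the level.
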(event Custom|RestartLervel
  (bind _returnvalue (Game|GetCurrentLevelName true))
  (Game|OpenLevel(byName) (Utilities|String|StringToName _returnvalue)))

(event Custom|SetSlimeLives
  (params (Lives :type Float%20%28single-precision%29))
  (Default|SlimeLiveUpdate (stale EventBeginPlay _returnvalue) Lives))

(event EventBeginPlay
  (if (Variables|Default|GetUIEnabled)
    (Utilities|FlowControl|Sequence
      (:then_0
        (bind _returnvalue (UserInterface|CreateWidget "/Game/Chillenium/UI/UI_slimes_available.UI_slimes_available_C" (Game|GetPlayerController 0)))
        (UserInterface|Viewport|AddtoViewport _returnvalue 0)))))

(event Input|ActionEvents|InputActionLeftClick
  (params (Key :type Key%20Structure))
  (bind _returnvalue (Game|GetPlayerController 0))
  (bind _hitresult (Game|Player|GetHitResultUnderCursorbyChannel _returnvalue "TraceTypeQuery1" false))
  (bind (_bblockinghit _binitialoverlap _time _distance _location _impactpoint _normal _impactnormal _physmat _hitactor) (Collision|BreakHitResult _hitresult))
  (bind _returnvalue_2 (Math|Transform|MakeTransform (Math|Vector|MakeVector (.x _impactpoint) 0.0 (.z _impactpoint))))
  ;[1 1 1] Spawn Object at cursor click
  (:Released
    (bind _outactors (Actor|GetAllActorsOfClass "/Game/Chillenium/Blueprints/BP_Change_Mouse_Icon.BP_Change_Mouse_Icon_C"))
    (bind _asbp_change_mouse_icon (Utilities|Casting|CastToBP_Change_Mouse_Icon (Utilities|Array|Get(acopy) _outactors))
      (:then
        (switch int (Variables|/Game/Chillenium/Blueprints/BP_Change_Mouse_Icon.BP_Change_Mouse_Icon_C|GetMouse%20Value _asbp_change_mouse_icon)
          (:1
            ;[1 1 1] Bomb
            (Game|SpawnActorfromClass "/Game/Chillenium/Items_For_Slime_To_Absorb/Bomb.Bomb_C" _returnvalue_2 "Undefined" 0 0)
            (bind _outactors_2 (Actor|GetAllActorsOfClass "/Game/Chillenium/Blueprints/BP_Change_Mouse_Icon.BP_Change_Mouse_Icon_C"))
            (bind _asbp_change_mouse_icon_2 (Utilities|Casting|CastToBP_Change_Mouse_Icon (Utilities|Array|Get(acopy) _outactors_2)))
            (Variables|/Game/Chillenium/Blueprints/BP_Change_Mouse_Icon.BP_Change_Mouse_Icon_C|SetMouse%20Value _asbp_change_mouse_icon_2 0))
          (:2
            ;[1 1 1] Wall
            (Game|SpawnActorfromClass "/Game/Chillenium/Items_For_Slime_To_Absorb/Wall_Slime_Trigger.Wall_Slime_Trigger_C" _returnvalue_2 "Undefined" 0 0)
            (bind _outactors_3 (Actor|GetAllActorsOfClass "/Game/Chillenium/Blueprints/BP_Change_Mouse_Icon.BP_Change_Mouse_Icon_C"))
            (bind _asbp_change_mouse_icon_3 (Utilities|Casting|CastToBP_Change_Mouse_Icon (Utilities|Array|Get(acopy) _outactors_3)))
            (Variables|/Game/Chillenium/Blueprints/BP_Change_Mouse_Icon.BP_Change_Mouse_Icon_C|SetMouse%20Value _asbp_change_mouse_icon_3 0))
          (:3
            ;[1 1 1] Comment
            (Game|SpawnActorfromClass "/Game/Chillenium/Items_For_Slime_To_Absorb/Call_Bounce.Call_Bounce_C" _returnvalue_2 "Undefined" 0 0)
            (bind _outactors_4 (Actor|GetAllActorsOfClass "/Game/Chillenium/Blueprints/BP_Change_Mouse_Icon.BP_Change_Mouse_Icon_C"))
            (bind _asbp_change_mouse_icon_4 (Utilities|Casting|CastToBP_Change_Mouse_Icon (Utilities|Array|Get(acopy) _outactors_4)))
            (Variables|/Game/Chillenium/Blueprints/BP_Change_Mouse_Icon.BP_Change_Mouse_Icon_C|SetMouse%20Value _asbp_change_mouse_icon_4 0))
          (:4
            ;[1 1 1] Comment
            (Game|SpawnActorfromClass "/Game/Chillenium/Items_For_Slime_To_Absorb/AcidSlime.AcidSlime_C" _returnvalue_2 "Undefined" 0 0)
            (bind _outactors_5 (Actor|GetAllActorsOfClass "/Game/Chillenium/Blueprints/BP_Change_Mouse_Icon.BP_Change_Mouse_Icon_C"))
            (bind _asbp_change_mouse_icon_5 (Utilities|Casting|CastToBP_Change_Mouse_Icon (Utilities|Array|Get(acopy) _outactors_5)))
            (Variables|/Game/Chillenium/Blueprints/BP_Change_Mouse_Icon.BP_Change_Mouse_Icon_C|SetMouse%20Value _asbp_change_mouse_icon_5 0))
          (:5
            ;[1 1 1] Bridge
            (Game|SpawnActorfromClass "/Game/Chillenium/Items_For_Slime_To_Absorb/Bridge_Slime_Trigger1.Bridge_Slime_Trigger1_C" _returnvalue_2 "AlwaysSpawn" 0 0)
            (bind _outactors_6 (Actor|GetAllActorsOfClass "/Game/Chillenium/Blueprints/BP_Change_Mouse_Icon.BP_Change_Mouse_Icon_C"))
            (bind _asbp_change_mouse_icon_6 (Utilities|Casting|CastToBP_Change_Mouse_Icon (Utilities|Array|Get(acopy) _outactors_6)))
            (Variables|/Game/Chillenium/Blueprints/BP_Change_Mouse_Icon.BP_Change_Mouse_Icon_C|SetMouse%20Value _asbp_change_mouse_icon_6 0))))
      (:CastFailed
        (Development|PrintString "fail")))))

(fn ConstructionScript)