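; BP_Win_Level_01 is the level goal trigger that counts surviving slimes and opens Level_02 on reaching the win threshold.
; When a slime's capsule overlaps its Box, it destroys the slime, increments SlimeSurvivedToWin and checks for equality with ValueWinCondition.
; An unfinished lose check on Tick compares the spawner's SlimeLives to that threshold once all slimes have spawned, but acts on no result.
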(event OnComponentBeginOverlap(Box)
  (params (OverlappedComponent :type Primitive%20Component%20Object%20Reference) (OtherActor :type Actor%20Object%20Reference) (OtherComp :type Primitive%20Component%20Object%20Reference) (OtherBodyIndex :type Integer) (bFromSweep :type Boolean) (SweepResult :type Hit%20Result%20Structure%20%28by%20ref%29))
  ;[1 1 1] Win
  (bind _asbp_slime (Utilities|Casting|CastToBP_Slime OtherActor))
  (if (== (Variables|/Script/Engine.Character|GetCapsuleComponent _asbp_slime) OtherComp)
    (Actor|DestroyActor _asbp_slime)
    (bind _output_get (Variables|Default|SetSlime%20Survived%20to%20Win (+ (Variables|Default|GetSlime%20Survived%20to%20Win) 1.0)))
    (Math|Float|CompareFloat _output_get (Variables|Default|GetValue%20Win%20Condition)
      (:==
        (Game|OpenLevel(byName) "Level_02")))))

(event EventTick
  (params (DeltaSeconds :type Float%20%28single-precision%29))
  ;[1 1 1] Lose Condition
  (bind _outactors (Actor|GetAllActorsOfClass "/Game/Chillenium/Blueprints/BP_Spawn_Slime.BP_Spawn_Slime_C"))
  (bind _asbp_spawn_slime (Utilities|Casting|CastToBP_Spawn_Slime (Utilities|Array|Get(acopy) _outactors)))
  (if (Variables|/Game/Chillenium/Blueprints/BP_Spawn_Slime.BP_Spawn_Slime_C|GetAll%20Slime%20Spawned _asbp_spawn_slime)
    (Math|Float|CompareFloat (Variables|/Game/Chillenium/Blueprints/BP_Spawn_Slime.BP_Spawn_Slime_C|GetSlime%20Lives _asbp_spawn_slime) (Variables|Default|GetValue%20Win%20Condition))))

(fn ConstructionScript)